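; BP_ChipPlatform is a platform actor whose mesh height tracks a chip count.
; The construction script derives the height per chip by dividing the MinZ to MaxZ range by MaxChips.
; MoveOneStep instantly shifts the mesh by one chip's height, while RemoveChips moves it back down by Amount steps over a one-second interpolation.
; Neither event clamps to the range or stores a count, and nothing in this graph calls them.
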(event `MoveOneStep`
  (`SceneComponent.K2_AddRelativeLocation` (`self.platformMesh`) (`KismetMathLibrary.MakeVector` 0.0 0.0 (`self.HeightPerChip`)) false false))

(event `RemoveChips`
  (params (Amount :type Integer))
  (bind _platformmesh (`self.platformMesh`))
  (bind (_relativelocation_x _relativelocation_y _relativelocation_z) (`KismetMathLibrary.BreakVector` (`SceneComponent.RelativeLocation` _platformmesh)))
  (`KismetSystemLibrary.MoveComponentTo` _platformmesh (`KismetMathLibrary.MakeVector` _relativelocation_x _relativelocation_y (- _relativelocation_z (* (`self.HeightPerChip`) Amount))) (struct) false false 1.0))

(fn `UserConstructionScript`
  (set `self.HeightPerChip` (/ (- (`self.MaxZ`) (`self.MinZ`)) (`self.MaxChips`))))