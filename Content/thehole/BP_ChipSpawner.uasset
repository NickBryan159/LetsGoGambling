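; BP_ChipSpawner queues requested chips and spawns them one at a time as BP_SingleChip actors at its Spawner component's transform.
; AddChipsToSpawn adds to the pending count and, if idle, starts a looping timer whose interval spreads that batch over a short, amount-scaled duration.
; TrySpawnChip drains the count, then clears the timer.
; BeginPlay caches BP_ChipPlatform, but its MoveOneStep call is unconnected.
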(event `self.ReceiveBeginPlay`
  ; Init find platform
  (bind _returnvalue (`GameplayStatics.GetActorOfClass` "/Game/thehole/BP_ChipPlatform.BP_ChipPlatform_C"))
  (set `self.Ref_Platform` _returnvalue))

(event `TrySpawnChip`
  ; get pending chips and spawn each of them
  (if (> (`self.PendingChips`) 0)
    (`|SpawnActorFromClass` "/Game/thehole/BP_SingleChip.BP_SingleChip_C" (`SceneComponent.K2_GetComponentToWorld` (`self.Spawner`)) "Undefined" "MultiplyWithRoot" null null)
    (set `self.PendingChips` (- (`self.PendingChips`) 1))
    (else
      ; loop trigger chips spawn
      (`KismetSystemLibrary.K2_ClearAndInvalidateTimerHandle` (`self.SpawnTimer`)))))

(event `AddChipsToSpawn`
  (params (Amount :type Integer))
  (bind _returnvalue (`KismetMathLibrary.Conv_IntToDouble` Amount))
  ; Receive call to add a chip
  (set `self.PendingChips` (+ Amount (`self.PendingChips`)))
  (if (not (`KismetSystemLibrary.K2_IsTimerActiveHandle` (`self.SpawnTimer`)))
    ; loop trigger chips spawn
    ;; how many sec per chip
    (bind _returnvalue_2 (`KismetSystemLibrary.K2_SetTimerDelegate` (delegate `TrySpawnChip`) (`KismetMathLibrary.FMax` (/ (`KismetMathLibrary.MapRangeClamped` _returnvalue 10.0 200.0 1.0 3.0) _returnvalue) 0.01) true))
    (set `self.SpawnTimer` _returnvalue_2)))

(fn `UserConstructionScript`)