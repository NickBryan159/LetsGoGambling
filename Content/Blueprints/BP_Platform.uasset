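; BP_Platform is a platform actor that rises or sinks on command and triggers the win screen at the top.
; MoveUp and MoveDown each play a timeline that lerps from the current location each update, so offsets accumulate, with larger upward than downward steps.
; When an upward move finishes at or above a hardcoded height, it calls YouWin on the first WBP_HUD found.
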(event `self.ReceiveTick`
  (params (DeltaSeconds :type "Float (single-precision)")))

(event `Key|E`
  (params (Key :type "Key Structure")))

(event `MoveUp`
  (bind (_returnvalue_x _returnvalue_y _returnvalue_z) (`KismetMathLibrary.BreakVector` (`self.K2_GetActorLocation`)))
  (bind _returnvalue (`self.K2_GetActorLocation`))
  (bind (_direction _alpha) (`Timeline|Timeline` :!via `PlayFromStart`)
    (:`Update`
      (`self.K2_SetActorLocation` (`KismetMathLibrary.VLerp` _returnvalue (+ _returnvalue (0.0 0.0 10.0)) _alpha)))
    (:`Finished`
      (if (>= _returnvalue_z 3100.0)
        (bind _foundwidgets (`WidgetBlueprintLibrary.GetAllWidgetsOfClass` "/Game/UI/WBP_HUD.WBP_HUD_C"))
        (`/Game/UI/WBP_HUD.YouWin` (`|GetArrayItem` _foundwidgets))))))

(event `MoveDown`
  (bind _returnvalue (`self.K2_GetActorLocation`))
  (bind (_direction _alpha) (`Timeline|Timeline_0` :!via `PlayFromStart`)
    (:`Update`
      (`self.K2_SetActorLocation` (`KismetMathLibrary.VLerp` _returnvalue (+ _returnvalue (0.0 0.0 -5.0)) _alpha)))))

(fn `UserConstructionScript`)