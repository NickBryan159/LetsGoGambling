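; Dice receiver actor that turns an overlapping BP_Dice into a random 1–6 roll and resolves the player's bet.
; On overlap it destroys the dice, shows the roll on its text and passes it to WBP_HUD.
; A roll matching the HUD's CurrentBet moves BP_Platform and this actor up; otherwise both move down.
; Timelines lerp this actor from its current location each update, so offsets accumulate.
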(event `self.ReceiveActorBeginOverlap`
  (params (OtherActor :type "Actor Object Reference"))
  (bind _returnvalue (`self.K2_GetActorLocation`))
  (bind _returnvalue_2 (`self.K2_GetActorLocation`))
  (bind _asbp_dice (cast `/Game/Blueprints/BP_Dice` OtherActor))
  (`self.K2_DestroyActor` _asbp_dice)
  (bind _output_get (set `self.randomResult` (`KismetMathLibrary.RandomIntegerInRange` 1 6)))
  (`TextRenderComponent.K2_SetText` (`self.OutputText`) (`KismetTextLibrary.Conv_IntToText` _output_get))
  (bind _foundwidgets (`WidgetBlueprintLibrary.GetAllWidgetsOfClass` "/Game/UI/WBP_HUD.WBP_HUD_C"))
  (bind _output (`|GetArrayItem` _foundwidgets))
  (`/Game/UI/WBP_HUD.UpdateRoll` _output (`self.randomResult`))
  (bind _returnvalue_3 (`GameplayStatics.GetActorOfClass` "/Game/Blueprints/BP_Platform.BP_Platform_C"))
  (if (== (`/Game/UI/WBP_HUD.currentBet` _output) (`self.randomResult`))
    (`/Game/Blueprints/BP_Platform.MoveUp` _returnvalue_3)
    (bind (_direction _alpha) (`Timeline|Timeline` :!via `PlayFromStart`)
      (:`Update`
        (`self.K2_SetActorLocation` (`KismetMathLibrary.VLerp` _returnvalue_2 (+ _returnvalue_2 (0.0 0.0 10.0)) _alpha))))
    (else
      (`/Game/Blueprints/BP_Platform.MoveDown` _returnvalue_3)
      (bind (_direction_2 _alpha_2) (`Timeline|Timeline_0` :!via `PlayFromStart`)
        (:`Update`
          (`self.K2_SetActorLocation` (`KismetMathLibrary.VLerp` _returnvalue (+ _returnvalue (0.0 0.0 -5.0)) _alpha_2)))))))

(event `MoveUp`)

(event `MoveDown`)

(fn `UserConstructionScript`)