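; BP_Dice is a physics die that throws itself on BeginPlay with a mass-scaled impulse and random torque.
; GetSideNumber reads the top face by finding the highest mesh socket and mapping its name to a number.
; Logic to await near-zero velocity, send the roll to WBP_HUD and move BP_Platform up or down against the bet exists but is disconnected.
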(event `self.ReceiveBeginPlay`
  (`self.StartRoll`))

(event `self.ReceiveTick`
  (params (DeltaSeconds :type "Float (single-precision)")))

(event `Rolled`)

(fn `GetSideNumber`
  (returns (Value :type Integer))
  (locals (SideMaxHeight :type "Float (double-precision)") (SideMaxHeightName :type Name))
  (bind _value (`BlueprintMapLibrary.Map_Find` (`self.NameToNumMap`) (`local.SideMaxHeightName`)))
  (for _array_element (`SceneComponent.GetAllSocketNames` (`self.dice`))
    (bind (_returnvalue_x _returnvalue_y _returnvalue_z) (`KismetMathLibrary.BreakVector` (`SceneComponent.GetSocketLocation` (`self.dice`) _array_element)))
    (if (> _returnvalue_z (`local.SideMaxHeight`))
      (set `local.SideMaxHeight` _returnvalue_z)
      (set `local.SideMaxHeightName` _array_element)))
  (set `self.SideNumber` _value)
  (return _value))

(fn `StartRoll`
  (`PrimitiveComponent.AddImpulse` (`self.dice`) (+ (* (`SceneComponent.GetForwardVector` (`self.dice`)) (* (`PrimitiveComponent.GetMass` (`self.dice`)) (`self.ForwardStrength`))) (* (`SceneComponent.GetUpVector` (`self.dice`)) (* (`PrimitiveComponent.GetMass` (`self.dice`)) (`self.UpStrength`)))) "None" false)
  (`PrimitiveComponent.AddTorqueInDegrees` (`self.dice`) (* (`KismetMathLibrary.RandomUnitVector`) (`PrimitiveComponent.GetMass` (`self.dice`)) (`self.TorqueStrength`)) "None" false)
  (`self.Rolled`))

(fn `UserConstructionScript`)