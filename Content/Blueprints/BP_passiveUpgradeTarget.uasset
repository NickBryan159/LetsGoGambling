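; BP_passiveUpgradeTarget is a shootable shop target that sells passive dice upgrades to the player for chips.
; When an overlapping actor tagged "Dice" arrives, it checks the player's dice count against MaxUpgrade and chips against CostMatrix, indexed by that count.
; A successful purchase disables the projectile's collision to prevent accidental ricochet bets, deducts chips, increments NumPassiveDice and updates the cost text.
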(event `self.ReceiveBeginPlay`
  (bind _asbp_shooter_character (cast `/Game/Variant_Shooter/Blueprints/BP_ShooterCharacter` (`GameplayStatics.GetPlayerCharacter` 0)))
  (set `self.playerRef` _asbp_shooter_character))

(event `self.ReceiveActorBeginOverlap`
  (params (OtherActor :type "Actor Object Reference"))
  (bind _playerref (`self.playerRef`))
  (bind _playerref_2 (`self.playerRef`))
  ; If overlapping actor is a dice projectile, remove Actor Collisions to prevent ricochets from unintentionally placing bets from hitting other dummies
  (if (and (`self.ActorHasTag` OtherActor "Dice") (< (`/Game/Variant_Shooter/Blueprints/BP_ShooterCharacter.numPassiveDice` _playerref) (`self.maxUpgrade`)) (>= (`/Game/Variant_Shooter/Blueprints/BP_ShooterCharacter.chips` _playerref) (`|GetArrayItem` (`self.costMatrix`) (`/Game/Variant_Shooter/Blueprints/BP_ShooterCharacter.numPassiveDice` _playerref))))
    (`self.SetActorEnableCollision` OtherActor false)
    ; Remove the chips from the player's chip total
    (`/Game/Variant_Shooter/Blueprints/BP_ShooterCharacter.ChangeChipAmount` _playerref_2 (* (`|GetArrayItem` (`self.costMatrix`) (`/Game/Variant_Shooter/Blueprints/BP_ShooterCharacter.numPassiveDice` _playerref_2)) -1))
    ; Increase the player's dice pool
    (bind _result (`/Engine/EditorBlueprintResources/StandardMacros.IncrementInt` (`/Game/Variant_Shooter/Blueprints/BP_ShooterCharacter.numPassiveDice` (`self.playerRef`)))
      (:`  `
        ; Update the cost text
        (`TextRenderComponent.K2_SetText` (`self.Cost`) (`KismetTextLibrary.Conv_StringToText` (`KismetStringLibrary.Concat_StrStr` (`KismetStringLibrary.Conv_IntToString` (`|GetArrayItem` (`self.costMatrix`) _result)) " Chips")))))))

(fn `UserConstructionScript`)