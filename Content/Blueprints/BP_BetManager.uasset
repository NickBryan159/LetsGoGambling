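; Dice-betting target that turns to face the player and teleports them to the range on overlap.
; A dice projectile hit validates the player's bet, then rolls 1 to 6 against their chosen number.
; A win adds six times the bet and queues chip spawns.
; A loss deducts it, calls the security spawner with the roll, and disables the target until RevealCube restores it.
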(event `self.ReceiveBeginPlay`
  (bind _returnvalue (`GameplayStatics.GetActorOfClass` "/Game/Security/BP_SecuritySpawner.BP_SecuritySpawner_C"))
  (set `self.SecuritySpawner` _returnvalue)
  (set `self.GambleText` (`TextRenderComponent.Text` (`self.Instruction Text`)))
  (bind _returnvalue_2 (`GameplayStatics.GetActorOfClass` "/Game/Variant_Shooter/Blueprints/BP_ShooterCharacter.BP_ShooterCharacter_C"))
  (set `self.player` _returnvalue_2))

(event `self.ReceiveActorBeginOverlap`
  (params (OtherActor :type "Actor Object Reference"))
  (if (`self.ActorHasTag` OtherActor "Player")
    ; Teleport the Player to the Range
    (`self.K2_SetActorLocation` OtherActor (500.0 11030.0 380.0) false false)
    (else
      ; If the overlapping actor is a dice projectile...
      (if (`self.ActorHasTag` OtherActor "Dice")
        ; Check to see if the player can bet:
        ; - If the amount of chips bet is within the player's budget (their chip total)
        ; - If the player has chosen a number...
        ; - If the bet is at or above the bet minimum (10 chips)
        (bind _asbp_shooter_character (cast `/Game/Variant_Shooter/Blueprints/BP_ShooterCharacter` (`GameplayStatics.GetPlayerCharacter` 0)))
        (bind _betchipamount (`/Game/Variant_Shooter/Blueprints/BP_ShooterCharacter.betChipAmount` _asbp_shooter_character))
        (if (and (and (>= (`/Game/Variant_Shooter/Blueprints/BP_ShooterCharacter.chips` _asbp_shooter_character) _betchipamount) (>= _betchipamount 10)) (> (`/Game/Variant_Shooter/Blueprints/BP_ShooterCharacter.numBetOn` _asbp_shooter_character) 0))
          ; Destroy the dice projectile
          (`self.K2_DestroyActor` OtherActor)
          ; Get a random number
          (bind _output_get (set `self.randomResult` (`KismetMathLibrary.RandomIntegerInRange` 1 6)))
          ; Update Output text
          (`TextRenderComponent.K2_SetText` (`self.OutputText`) (`KismetTextLibrary.Conv_IntToText` _output_get))
          ; Determine outcome of the roll
          (if (== (`self.randomResult`) (`/Game/Variant_Shooter/Blueprints/BP_ShooterCharacter.numBetOn` _asbp_shooter_character))
            ; Add gained chips
            (bind _asbp_shooter_character_2 (cast `/Game/Variant_Shooter/Blueprints/BP_ShooterCharacter` (`GameplayStatics.GetPlayerCharacter` 0)))
            (bind _returnvalue (* (`/Game/Variant_Shooter/Blueprints/BP_ShooterCharacter.betChipAmount` _asbp_shooter_character_2) 6))
            (`/Game/Variant_Shooter/Blueprints/BP_ShooterCharacter.ChangeChipAmount` _asbp_shooter_character_2 _returnvalue)
            (`/Game/thehole/BP_ChipSpawner.AddChipsToSpawn` (`self.chipSpawnerRef`) _returnvalue)
            (else
              ; Remove lost chips
              (bind _asbp_shooter_character_3 (cast `/Game/Variant_Shooter/Blueprints/BP_ShooterCharacter` (`GameplayStatics.GetPlayerCharacter` 0)))
              (`/Game/Variant_Shooter/Blueprints/BP_ShooterCharacter.ChangeChipAmount` _asbp_shooter_character_3 (* (`/Game/Variant_Shooter/Blueprints/BP_ShooterCharacter.betChipAmount` _asbp_shooter_character_3) -1))
              ; Spawn enemies and disable further betting
              (`/Game/Security/BP_SecuritySpawner.SpawnAEnemy` (`self.SecuritySpawner`) (`self.randomResult`))
              (`SceneComponent.SetHiddenInGame` (`self.Cube`) true false)
              (`TextRenderComponent.K2_SetText` (`self.Instruction Text`) (`self.ClearText`))
              (`self.SetActorEnableCollision` false))))))))

(event `self.ReceiveTick`
  (params (DeltaSeconds :type "Float (single-precision)"))
  (bind (_returnvalue_roll _returnvalue_pitch _returnvalue_yaw) (`KismetMathLibrary.BreakRotator` (`KismetMathLibrary.FindLookAtRotation` (`self.K2_GetActorLocation`) (`self.K2_GetActorLocation` (`GameplayStatics.GetPlayerCharacter` 0)))))
  ; Always Keep the Better Looking at the player for ease of betting
  (`self.K2_SetActorRotation` (`KismetMathLibrary.MakeRotator` 0.0 0.0 _returnvalue_yaw)))

(event `RevealCube`
  ; Re-enable the cube
  (`SceneComponent.SetHiddenInGame` (`self.Cube`) false false)
  (`TextRenderComponent.K2_SetText` (`self.Instruction Text`) (`KismetTextLibrary.Conv_StringToText` (`KismetStringLibrary.Concat_StrStr` (`KismetStringLibrary.Concat_StrStr` "Shoot Me \nto Gamble! \n \nEnter to  \nPlace a Bet! \n \nCurrent Bet: \n" (`KismetStringLibrary.Conv_IntToString` (`/Game/Variant_Shooter/Blueprints/BP_ShooterCharacter.betChipAmount` (`self.player`)))) " Chips")))
  (`TextRenderComponent.K2_SetText` (`self.OutputText`) (`KismetTextLibrary.Conv_StringToText` ""))
  (`self.SetActorEnableCollision` true))

(fn `UserConstructionScript`)