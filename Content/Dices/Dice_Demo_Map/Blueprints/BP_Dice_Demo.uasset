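; BP_Dice_Demo is a showcase actor for the dice demo map that spins a collection of dice meshes, from steampunk and sci-fi styles to DnD polyhedrals.
; Each Tick adds a world-space yaw rotation to all dice components, scaled by DeltaSeconds and RotationSpeed with a slight random jitter.
; An alternative local-rotation version of the same spin is left unconnected.
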(event `self.ReceiveTick`
  (params (DeltaSeconds :type "Float (single-precision)"))
  (`SceneComponent.K2_AddWorldRotation` (`self.SM_Dice_Steampunk_3`) (`KismetMathLibrary.MakeRotator` 0.0 0.0 (* DeltaSeconds (* (`self.Rotation Speed`) (`KismetMathLibrary.RandomFloatInRange` 0.9 1.1)))) false false)
  (`SceneComponent.K2_AddWorldRotation` (`self.SM_Dice_2`) (`KismetMathLibrary.MakeRotator` 0.0 0.0 (* DeltaSeconds (* (`self.Rotation Speed`) (`KismetMathLibrary.RandomFloatInRange` 0.9 1.1)))) false false)
  (`SceneComponent.K2_AddWorldRotation` (`self.SM_Dice_3`) (`KismetMathLibrary.MakeRotator` 0.0 0.0 (* DeltaSeconds (* (`self.Rotation Speed`) (`KismetMathLibrary.RandomFloatInRange` 0.9 1.1)))) false false)
  (`SceneComponent.K2_AddWorldRotation` (`self.SM_Dice_Hollow`) (`KismetMathLibrary.MakeRotator` 0.0 0.0 (* DeltaSeconds (* (`self.Rotation Speed`) (`KismetMathLibrary.RandomFloatInRange` 0.9 1.1)))) false false)
  (`SceneComponent.K2_AddWorldRotation` (`self.SM_Dice_Sci-Fi`) (`KismetMathLibrary.MakeRotator` 0.0 0.0 (* DeltaSeconds (* (`self.Rotation Speed`) (`KismetMathLibrary.RandomFloatInRange` 0.9 1.1)))) false false)
  (`SceneComponent.K2_AddWorldRotation` (`self.SM_Dice_Spider`) (`KismetMathLibrary.MakeRotator` 0.0 0.0 (* DeltaSeconds (* (`self.Rotation Speed`) (`KismetMathLibrary.RandomFloatInRange` 0.9 1.1)))) false false)
  (`SceneComponent.K2_AddWorldRotation` (`self.SM_Dice_Steampunk_1`) (`KismetMathLibrary.MakeRotator` 0.0 0.0 (* DeltaSeconds (* (`self.Rotation Speed`) (`KismetMathLibrary.RandomFloatInRange` 0.9 1.1)))) false false)
  (`SceneComponent.K2_AddWorldRotation` (`self.SM_Dice_Steampunk_2`) (`KismetMathLibrary.MakeRotator` 0.0 0.0 (* DeltaSeconds (* (`self.Rotation Speed`) (`KismetMathLibrary.RandomFloatInRange` 0.9 1.1)))) false false)
  (`SceneComponent.K2_AddWorldRotation` (`self.SM_Dice_1`) (`KismetMathLibrary.MakeRotator` 0.0 0.0 (* DeltaSeconds (* (`self.Rotation Speed`) (`KismetMathLibrary.RandomFloatInRange` 0.9 1.1)))) false false)
  (`SceneComponent.K2_AddWorldRotation` (`self.SM_Dices_DND_D10a`) (`KismetMathLibrary.MakeRotator` 0.0 0.0 (* DeltaSeconds (* (`self.Rotation Speed`) (`KismetMathLibrary.RandomFloatInRange` 0.9 1.1)))) false false)
  (`SceneComponent.K2_AddWorldRotation` (`self.SM_Dices_DND_D10b`) (`KismetMathLibrary.MakeRotator` 0.0 0.0 (* DeltaSeconds (* (`self.Rotation Speed`) (`KismetMathLibrary.RandomFloatInRange` 0.9 1.1)))) false false)
  (`SceneComponent.K2_AddWorldRotation` (`self.SM_Dices_DND_D12`) (`KismetMathLibrary.MakeRotator` 0.0 0.0 (* DeltaSeconds (* (`self.Rotation Speed`) (`KismetMathLibrary.RandomFloatInRange` 0.9 1.1)))) false false)
  (`SceneComponent.K2_AddWorldRotation` (`self.SM_Dices_DND_D20`) (`KismetMathLibrary.MakeRotator` 0.0 0.0 (* DeltaSeconds (* (`self.Rotation Speed`) (`KismetMathLibrary.RandomFloatInRange` 0.9 1.1)))) false false)
  (`SceneComponent.K2_AddWorldRotation` (`self.SM_Dices_DND_D4`) (`KismetMathLibrary.MakeRotator` 0.0 0.0 (* DeltaSeconds (* (`self.Rotation Speed`) (`KismetMathLibrary.RandomFloatInRange` 0.9 1.1)))) false false)
  (`SceneComponent.K2_AddWorldRotation` (`self.SM_Dices_DND_D6`) (`KismetMathLibrary.MakeRotator` 0.0 0.0 (* DeltaSeconds (* (`self.Rotation Speed`) (`KismetMathLibrary.RandomFloatInRange` 0.9 1.1)))) false false)
  (`SceneComponent.K2_AddWorldRotation` (`self.SM_Dices_DND_D8`) (`KismetMathLibrary.MakeRotator` 0.0 0.0 (* DeltaSeconds (* (`self.Rotation Speed`) (`KismetMathLibrary.RandomFloatInRange` 0.9 1.1)))) false false))

(fn `UserConstructionScript`)