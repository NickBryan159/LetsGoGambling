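; BP_SecuritySpawner spawns BP_Security enemies and tracks how many remain alive.
; SpawnAEnemy places the requested number of enemies at random points inside the SpawnArea box, always spawning regardless of collision.
; RegisterEnemy and UnregisterEnemy adjust the live count, and when it drops to zero the spawner finds BP_BetManager and calls RevealCube.
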(event `self.ReceiveBeginPlay`
  (set `self.CurrentEnemyCount` 0))

(event `SpawnAEnemy`
  (params (EnemyToSpawn :type Integer))
  (bind _spawnarea (`self.SpawnArea`))
  ; Spawn Enemy
  (for _ (range 1 (+ EnemyToSpawn 1))
    (`|SpawnActorFromClass` "/Game/Security/BP_Security.BP_Security_C" (`KismetMathLibrary.MakeTransform` (`KismetMathLibrary.RandomPointInBoundingBox` (`SceneComponent.K2_GetComponentLocation` _spawnarea) (`BoxComponent.GetScaledBoxExtent` _spawnarea))) "AlwaysSpawn" "MultiplyWithRoot" null null)))

(event `RegisterEnemy`
  ; Register Enemy
  (`/Engine/EditorBlueprintResources/StandardMacros.IncrementInt` (`self.CurrentEnemyCount`)))

(event `UnregisterEnemy`
  ; Unregister Enemy
  (`/Engine/EditorBlueprintResources/StandardMacros.DecrementInt` (`self.CurrentEnemyCount`)
    (:`  `
      (if (== (`self.CurrentEnemyCount`) 0)
        (bind _returnvalue (`GameplayStatics.GetActorOfClass` "/Game/Blueprints/BP_BetManager.BP_BetManager_C"))
        (`/Game/Blueprints/BP_BetManager.RevealCube` _returnvalue)))))

(fn `UserConstructionScript`)