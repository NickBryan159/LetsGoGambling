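; BP_Security_JJ is an AI-controlled melee security enemy that punches the player and can be killed by dice projectiles.
; A looping timer started on possession writes the blackboard's InAttackRange flag from player distance.
; TriggerMeleeAttack plays a punch montage behind an IsAttacking guard, while a separate event sphere-traces forward to damage BP_ShooterCharacter.
; Damage-enabled dice hits reduce health, and it registers with BP_SecuritySpawner on BeginPlay, unregistering on death.
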(event `self.ReceiveBeginPlay`
  ; init
  (set `self.CurrentHealth` (`self.MaxHealth`))
  (bind _returnvalue (`GameplayStatics.GetActorOfClass` "/Game/Security/BP_SecuritySpawner.BP_SecuritySpawner_C"))
  (`/Game/Security/BP_SecuritySpawner.RegisterEnemy` _returnvalue))

(event `CheckDistance`
  (bind _returnvalue (`AIBlueprintHelperLibrary.GetBlackboard` (`AIBlueprintHelperLibrary.GetAIController` self)))
  ; check the distance to player
  (`/Engine/EditorBlueprintResources/StandardMacros.IsValid` _returnvalue
    (:`Is Valid`
      (`BlackboardComponent.SetValueAsBool` _returnvalue "InAttackRange" (< (`self.GetDistanceTo` (`GameplayStatics.GetPlayerCharacter` 0) self) (`self.AttackRange`))))))

(event `self.ReceivePossessed`
  (params (NewController :type "Controller Object Reference"))
  ; loop trigger
  (`KismetSystemLibrary.Delay` 0.1)
  (`KismetSystemLibrary.K2_SetTimerDelegate` (delegate `CheckDistance`) 0.2 true))

(event `EventExcuteAttack`
  (bind _returnvalue (+ (`self.K2_GetActorLocation` self) (0.0 0.0 50.0)))
  ; Execute attack
  (bind (_outhit _returnvalue_2) (`KismetSystemLibrary.SphereTraceSingleForObjects` _returnvalue (+ (* (`self.GetActorForwardVector` self) (150.0 150.0 150.0)) _returnvalue) 30.0 (`|MakeArray` "ObjectTypeQuery3" :!type "EObjectTypeQuery Enum") false (`|MakeArray` self :!type "Actor Object Reference") "ForDuration"))
  (if _returnvalue_2
    (bind _asbp_shooter_character (cast `/Game/Variant_Shooter/Blueprints/BP_ShooterCharacter` (`.HitActor` (`GameplayStatics.BreakHitResult` _outhit))))
    (`/Game/Variant_Shooter/Blueprints/BP_ShooterCharacter.TakeDamage` _asbp_shooter_character 10.0)))

(event `TriggerMeleeAttack`
  ; Comment
  (if (not (`self.bIsAttacking`))
    (set `self.bIsAttacking` true)
    (bind _returnvalue (`self.PlayAnimMontage` "/Game/Security/Cross_Punch_Anim_Montage.Cross_Punch_Anim_Montage"))
    (`KismetSystemLibrary.Delay` _returnvalue)
    (set `self.bIsAttacking` false)))

(event `self.CapsuleComponent.OnComponentHit`
  (params (HitComponent :type "PrimitiveComponent Object Reference") (OtherActor :type "Actor Object Reference") (OtherComp :type "PrimitiveComponent Object Reference") (NormalImpulse :type "Vector Structure") (Hit :type "HitResult Structure (by ref)"))
  ; hit and call damage event
  (bind _asbp_shooter_projectile_dice (cast `/Game/Variant_Shooter/Blueprints/Pickups/Projectiles/BP_ShooterProjectile_Dice` OtherActor))
  (if (`/Game/Variant_Shooter/Blueprints/Pickups/Projectiles/BP_ShooterProjectile_Dice.CanDealDamage` _asbp_shooter_projectile_dice)
    (`KismetSystemLibrary.IsObjectOfSoftClass` OtherActor "/Game/Variant_Shooter/Blueprints/Pickups/Projectiles/BP_ShooterProjectile_Dice.BP_ShooterProjectile_Dice_C"
      (:`True`
        (`self.TakeDamage` 5.0)))))

(event `TakeDamage`
  (params (damage :type "Float (double-precision)"))
  ; take damage
  (bind _output_get (set `self.CurrentHealth` (- (`self.CurrentHealth`) damage)))
  (if (<= _output_get 0.0)
    (bind _returnvalue (`GameplayStatics.GetActorOfClass` "/Game/Security/BP_SecuritySpawner.BP_SecuritySpawner_C"))
    (`/Game/Security/BP_SecuritySpawner.UnregisterEnemy` _returnvalue)
    (`self.K2_DestroyActor`)))

(fn `UserConstructionScript`)